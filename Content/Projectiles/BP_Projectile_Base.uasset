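; Base projectile actor that flies at a configurable speed and gravity, optionally homing on a target.
; The construction script configures the movement component, including homing on the target's root component when enabled.
; On BeginPlay it ignores its owner during movement and aims its velocity at any valid target.
; On hit it calls the OnprojectileImpact dispatcher, spawns a Niagara explosion and impact sound, then destroys itself.
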(event `self.ReceiveBeginPlay`
  (`PrimitiveComponent.IgnoreActorWhenMoving` (`self.Projectile_Collision`) (`self.GetOwner`) true)
  (`self.Target`
    (:`then`
      (`self.RotateToTarget`))
    (:`else`)))

(event `RotateToTarget`
  (set `MovementComponent.Velocity` (* (`KismetMathLibrary.GetDirectionUnitVector` (`self.K2_GetActorLocation`) (`self.K2_GetActorLocation` (`self.Target`))) (`self.Speed`)) (`self.ProjectileMovement`)))

(event `self.Projectile_Collision.OnComponentHit`
  (params (HitComponent :type "PrimitiveComponent Object Reference") (OtherActor :type "Actor Object Reference") (OtherComp :type "PrimitiveComponent Object Reference") (NormalImpulse :type "Vector Structure") (Hit :type "HitResult Structure (by ref)"))
  (bind (_bblockinghit _binitialoverlap _time _distance _location) (`GameplayStatics.BreakHitResult` Hit))
  (`self.OnprojectileImpact` OtherActor Hit)
  (`NiagaraFunctionLibrary.SpawnSystemAtLocation` (`self.Niagara Explosion`) _location)
  (`GameplayStatics.PlaySoundAtLocation` (`self.Impact Sound`) _location (struct) 1.0 1.0 0.0 null null null null)
  (`self.K2_DestroyActor`))

(fn `UserConstructionScript`
  (bind _projectilemovement (`self.ProjectileMovement`))
  (set `ProjectileMovementComponent.InitialSpeed` (`self.Speed`) _projectilemovement)
  (set `ProjectileMovementComponent.MaxSpeed` (`self.Speed`) _projectilemovement)
  (set `ProjectileMovementComponent.ProjectileGravityScale` (`self.Gravity`) _projectilemovement)
  (`self.Target`
    (:`then`
      (if (`self.IsHoming`)
        (set `ProjectileMovementComponent.bIsHomingProjectile` true _projectilemovement)
        (set `ProjectileMovementComponent.HomingTargetComponent` (`Actor.RootComponent` (`self.Target`)) _projectilemovement)))
    (:`else`)))