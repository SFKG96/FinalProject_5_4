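; BP_Enemy is a demo enemy that periodically attacks pawns ahead of it and can take damage, heal and die.
; A looping timer fires a forward sphere trace, sending damage info to the hit actor with an explosion effect on success.
; BPCDamageSystem handles health, feeding a health bar widget and driving ragdoll death and block/response debug prints.
; It also contains dash-location helpers and player-input setup, but nothing here calls the dash functions.
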(event `self.ReceiveBeginPlay`
  ;[1 1 1] Damage System Implaction
  (`|ExecutionSequence`
    (:`then_0`
      ;[1 1 1] Basic Move Input
      (bind _asplayer_controller (cast `PlayerController` (`self.GetController`)))
      (bind _returnvalue (pcsubsystem `EnhancedInputLocalPlayerSubsystem` _asplayer_controller))
      (`/Engine/EditorBlueprintResources/StandardMacros.IsValid` _returnvalue
        (:`Is Valid`
          (`EnhancedInputSubsystemInterface.AddMappingContext` _returnvalue "/Game/TopDown/Input/Actions/IMC_WASD_Move.IMC_WASD_Move" 0 (struct))
          (set `PlayerController.bShowMouseCursor` true (`GameplayStatics.GetPlayerController` 0)))))
    (:`then_1`
      (`KismetSystemLibrary.K2_SetTimerDelegate` (delegate `EnemyAttack`) 2.0 true))
    (:`then_2`
      (bind _returnvalue_2 (`|CreateWidget` "/Game/DamageSystem/W_HealthBar.W_HealthBar_C" null self))
      (`WidgetComponent.SetWidget` (`self.HealthBarWidget`) _returnvalue_2))))

(event `EnemyAttack`
  (bind _returnvalue (`self.K2_GetActorLocation`))
  ;[1 1 1] Damage System Implaction
  (if (not (`/Game/DamageSystem/BPC_DamageSystem.IsDead` (`self.BPC_DamageSystem`)))
    (bind (_outhit _returnvalue_2) (`KismetSystemLibrary.SphereTraceSingleForObjects` :`Start` _returnvalue :`End` (+ _returnvalue (* (`self.GetActorForwardVector`) 100.0)) :`Radius` 20.0 :`ObjectTypes` (`|MakeArray` "ObjectTypeQuery3" :!type "EObjectTypeQuery Enum") :`DrawDebugType` "ForDuration" :`TraceColor` (struct :`R` 1.0 :`G` 0.94788 :`A` 1.0) :`TraceHitColor` (struct :`R` 0.52702 :`B` 1.0 :`A` 1.0) :`DrawTime` 1.0))
    (if _returnvalue_2
      (bind (_bblockinghit _binitialoverlap _time _distance _location _impactpoint _normal _impactnormal _physmat _hitactor) (`GameplayStatics.BreakHitResult` _outhit))
      (bind _wasdamaged (message `/Game/DamageSystem/BPI_Damagable.TakeDamage` _hitactor (make `/Game/DamageSystem/S_DamageInfo` 5.0 "NewEnumerator1" "NewEnumerator1")))
      (if _wasdamaged
        (`GameplayStatics.SpawnEmitterAtLocation` "/Game/StarterContent/Particles/P_Explosion.P_Explosion" _location)))))

(event `OnDeath_Event`
  (bind _mesh (`self.Mesh`))
  ;[1 1 1] Basic Take Damage Funcation (For demo)
  (`PrimitiveComponent.SetSimulatePhysics` _mesh true)
  (`PrimitiveComponent.SetCollisionEnabled` _mesh "QueryAndPhysics"))

(event `Blocked`
  (params (CanBeParried :type Boolean))
  ;[1 1 1] Basic Take Damage Funcation (For demo)
  (`KismetSystemLibrary.PrintString` "Blocked"))

(event `DamageResponse`
  (params (DamageResponse :type "/Game/DamageSystem/E_DamageRespones Enum" :default "NewEnumerator0"))
  ;[1 1 1] Basic Take Damage Funcation (For demo)
  (`KismetSystemLibrary.PrintString` (`|GetEnumeratorNameAsString` DamageResponse)))

(fn `CalculateDashTargetLocation`
  (returns (Location :type "Vector Structure"))
  (bind _returnvalue (`self.GetLastMovementInputVector`))
  (return (+ (`self.K2_GetActorLocation`) (* (`KismetMathLibrary.SelectVector` (`self.GetActorForwardVector`) _returnvalue (== _returnvalue (0.0 0.0 0.0))) (`self.MaxDashDistance`)))))

(fn `GetCurrentHealth`
  (returns (CurrentHealth :type "Float (double-precision)"))
  (return (`/Game/DamageSystem/BPC_DamageSystem.CurrentHealth` (`self.BPC_DamageSystem`))))

(fn `GetFurthestLocationAlongRoute`
  (params (Start :type "Vector Structure") (End :type "Vector Structure"))
  (returns (Location :type "Vector Structure"))
  (locals (Diracton :type "Vector Structure" :default (0.0 0.0 0.0)) (CapsuleDiamtor :type "Float (double-precision)") (CapsuleCount :type Integer))
  (bind (_outradius _outhalfheight) (`CapsuleComponent.GetUnscaledCapsuleSize` (`self.CapsuleComponent`)))
  (set `local.Diracton` (`KismetMathLibrary.GetDirectionUnitVector` Start End))
  (bind _output_get (set `local.CapsuleDiamtor` (* (`CapsuleComponent.CapsuleRadius` (`self.CapsuleComponent`)) 2.0)))
  (bind _output_get_2 (set `local.CapsuleCount` (/ (`KismetMathLibrary.Vector_Distance` Start End) _output_get)))
  (for _index (range (+ _output_get_2 1))
    (bind _output_get_3 (set `self.CurrentCapsuleLocation` (+ (`local.Start`) (* (- (`local.CapsuleCount`) _index) (`local.Diracton`) (`local.CapsuleDiamtor`)))))
    (bind _outhits (`KismetSystemLibrary.CapsuleTraceMultiForObjects` _output_get_3 _output_get_3 _outradius _outhalfheight (`|MakeArray` "ObjectTypeQuery1" "ObjectTypeQuery2" "ObjectTypeQuery3" "ObjectTypeQuery5" "ObjectTypeQuery6" :!type "EObjectTypeQuery Enum")))
    (bind _isvalid_ (`self.Is Valid Dash Location` (`self.CurrentCapsuleLocation`) _outhits))
    (if _isvalid_
      (return (`self.CurrentCapsuleLocation`))))
  (return (`self.DashStartLocation`)))

(fn `GetMaxHealth`
  (returns (MaxHealth :type "Float (double-precision)"))
  (return (`/Game/DamageSystem/BPC_DamageSystem.MaxHealth` (`self.BPC_DamageSystem`))))

(fn `Heal`
  (params (Amount_I_Heal :type "Float (double-precision)"))
  (returns (NewCurrentHealth :type "Float (double-precision)"))
  (bind _newcurrenthealth (`/Game/DamageSystem/BPC_DamageSystem.Heal` (`self.BPC_DamageSystem`) Amount_I_Heal))
  (return _newcurrenthealth))

(fn `Is Valid Dash Location`
  (params (Location :type "Vector Structure") (Hits :type "Array of HitResult Structure"))
  (returns (`IsValid?` :type Boolean))
  (bind (_outhit _returnvalue) (`KismetSystemLibrary.LineTraceSingle` Location (+ Location (0.0 0.0 -500.0)) "TraceTypeQuery1"))
  (if _returnvalue
    (if (`KismetArrayLibrary.Array_IsEmpty` Hits)
      (return true)
      (else
        (for _array_element Hits
          (if (`|EnumEquality` (`PrimitiveComponent.GetCollisionResponseToChannel` (`.HitComponent` (`GameplayStatics.BreakHitResult` _array_element)) "ECC_Pawn") "ECR_Block")
            (return false)))
        (return true)))
    (else
      (return false))))

(fn `TakeDamage`
  (params (DamageInfo :type "/Game/DamageSystem/S_DamageInfo Structure"))
  (returns (WasDamaged :type Boolean))
  (bind _wasdamaged (`/Game/DamageSystem/BPC_DamageSystem.TakeDamage` (`self.BPC_DamageSystem`) DamageInfo))
  (return _wasdamaged))

(fn `UserConstructionScript`
  (bind _bpc_damagesystem (`self.BPC_DamageSystem`))
  (set `self.AvailableDashCount` (`self.MaxDashCount`))
  (add `/Game/DamageSystem/BPC_DamageSystem.OnDeath` _bpc_damagesystem (`|CreateDelegate` :!event `OnDeath_Event`))
  (add `/Game/DamageSystem/BPC_DamageSystem.OnBlock` _bpc_damagesystem (`|CreateDelegate` :!event `Blocked`))
  (add `/Game/DamageSystem/BPC_DamageSystem.OnDamageResponse` _bpc_damagesystem (`|CreateDelegate` :!event `DamageResponse`)))