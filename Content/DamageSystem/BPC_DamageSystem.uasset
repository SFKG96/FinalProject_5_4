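; BPC_DamageSystem is a damage component that manages health, healing, blocking, invincibility frames and death for its owner.
; TakeDamage routes a DamageInfo struct through the CanBeDamaged macro into block, damage or no-damage outcomes.
; It fires OnBlock with parry eligibility, OnDeath at zero health, or OnDamageResponse when the hit interrupts.
; Heal clamps health to MaxHealth and only applies while alive.
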(fn `Heal`
  (params (Amount :type "Float (double-precision)"))
  (returns (NewCurrentHealth :type "Float (double-precision)"))
  (if (not (`self.IsDead`))
    (bind _output_get (set `self.CurrentHealth` (`KismetMathLibrary.FClamp` (+ Amount (`self.CurrentHealth`)) 0.0 (`self.MaxHealth`))))
    (return _output_get)))

(fn `TakeDamage`
  (params (DamageInfo :type "/Game/DamageSystem/S_DamageInfo Structure"))
  (returns (WasDamaged :type Boolean))
  (bind (_amountofdamage _damagetype _damagerespone _shoulddamageiframe _canbeblocked _canbeparried _shouldforceinterrupt) (break `/Game/DamageSystem/S_DamageInfo` DamageInfo))
  (`self.CanBeDamaged` _shoulddamageiframe _canbeblocked
    (:`BlockDamage`
      (`self.OnBlock` _canbeparried)
      (return false))
    (:`DoDamage`
      (bind _output_get (set `self.CurrentHealth` (- (`self.CurrentHealth`) _amountofdamage)))
      (if (<= _output_get 0.0)
        (set `self.IsDead` true)
        (`self.OnDeath`)
        (return true)
        (elif (or (`self.IsInterruptble`) _shouldforceinterrupt)
          (`self.OnDamageResponse` _damagerespone)
          (return true))))
    (:`NoDamage`
      (return false))))